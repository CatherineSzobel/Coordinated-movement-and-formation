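; RTS player controller that drives marquee unit selection and formation move commands, with the cursor shown.
; Left mouse forwards press, hold and release to the HUD, which supplies the selected units.
; Right click passes the hit location to C++ formation functions, then MoveFormation sends each unit its slot.
; E cycles four straight-line formations and re-issues the move from a zero origin; after any move, Tick snaps stationary selected units to a fixed rotation.
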(event `self.ReceiveTick`
  (params (DeltaSeconds :type "Float (single-precision)"))
  ;[1 1 1] Event tick
  (`|ExecutionSequence`
    (:`then_0`
      (if (`self.IsLeftMousePressed`)
        ;[1 1 1] Left mouse action
        (message `/Game/Blueprints/BP_RTSInterface.Marquees Hold` (`self.GetHUD`))))
    (:`then_1`
      ;[1 1 1] Rotate units
      (if (`self.HasGoneToPosition`)
        (bind _units (message `/Game/Blueprints/BP_RTSInterface.Grab Selected Units` (`self.GetHUD`)))
        (for _array_element _units
          (bind _asbp_base_units (cast `/Game/Blueprints/BP_BaseUnits` _array_element))
          (if (not (> (`KismetMathLibrary.VSize` (`MovementComponent.Velocity` (`Character.CharacterMovement` _asbp_base_units))) 0.0))
            (`self.K2_SetActorRotation` _asbp_base_units (struct :`Yaw` 180.0) false)))))))

(event `self.ReceiveBeginPlay`
  ;[1 1 1] Begin play
  (`WidgetBlueprintLibrary.SetInputMode_GameAndUIEx` self null "LockAlways" false)
  (set `self.bShowMouseCursor` true)
  (set `self.formationType` "StraightLineVerticalRight"))

(event `Key|LeftMouseButton`
  (params (Key :type "Key Structure"))
  (bind _returnvalue (`self.GetHUD`))
  ;[1 1 1] Left mouse action
  (:`Pressed`
    (set `self.IsLeftMousePressed` true)
    (message `/Game/Blueprints/BP_RTSInterface.Marquees Pressed` _returnvalue))
  (:`Released`
    (set `self.IsLeftMousePressed` false)
    (message `/Game/Blueprints/BP_RTSInterface.Marquees Released` _returnvalue)))

(event `Key|RightMouseButton`
  (params (Key :type "Key Structure"))
  ;[1 1 1] Make the selected units move
  (:`Pressed`
    (bind _output_get (set `self.RightClickPosition` (`.Location` (`GameplayStatics.BreakHitResult` (`self.GetHitResultUnderCursorByChannel` "TraceTypeQuery1")))))
    (bind _units (message `/Game/Blueprints/BP_RTSInterface.Grab Selected Units` (`self.GetHUD`)))
    ;;[1 1 1] c++ functions
    (`self.MakeFormation` _output_get _units)
    (`self.CallFormation`)
    (`self.MoveFormation` _units)))

(event `Key|E`
  (params (Key :type "Key Structure"))
  (:`Pressed`
    (switch `FormationType` (`self.formationType`)
      (:`StraightLineVerticalRight`
        (set `self.formationType` "StraightLineVerticalLeft"))
      (:`StraightLineVerticalLeft`
        (set `self.formationType` "StraightLineHorizontalUp"))
      (:`StraightLineHorizontalUp`
        (set `self.formationType` "StraightLineHorizontalDown"))
      (:`StraightLineHorizontalDown`
        (set `self.formationType` "StraightLineVerticalRight")))
    (bind _units (message `/Game/Blueprints/BP_RTSInterface.Grab Selected Units` (`self.GetHUD`)))
    (`self.MakeFormation` (0.0 0.0 0.0) _units)
    (`self.CallFormation`)
    (`self.MoveFormation` _units)))

(fn `CallFormatio`
  (bind _formationvector (`self.FormationVector`))
  (for (_ _array_index) _formationvector
    (`KismetSystemLibrary.DrawDebugCircle` (`|GetArrayItem` _formationvector _array_index) 10.0 12 (struct :`A` 1.0) 20.0 5.0)))

(fn `MoveFormation`
  (params (Units :type "Array of Actor Object Reference"))
  (for (_array_element _array_index) Units
    (message `/Game/Blueprints/BP_RTSInterface.Unit Move Command` _array_element (`|GetArrayItem` (`self.FormationVector`) _array_index)))
  (`KismetSystemLibrary.DrawDebugCircle` (0.0 0.0 0.0) 15.0 12 (struct :`R` 1.0 :`A` 1.0) 10.0 5.0 (0.0 1.0 0.0) (0.0 0.0 1.0) true)
  (`KismetArrayLibrary.Array_Clear` (`self.FormationVector`))
  (set `self.HasGoneToPosition` true))

(fn `UserConstructionScript`)