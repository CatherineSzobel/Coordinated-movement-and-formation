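; CameraPawn is a pawn that scrolls across the world along X and Y from player input.
; The LeftRight and TopDown axes apply world offsets on Y and X, scaled by ScrollSpeed and frame delta time.
; Screen-edge scrolling, which compares mouse position to the outer 2% of the viewport, is present but disconnected.
; The MouseX and MouseY events are empty, so only the axis inputs move the pawn.
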(event `InputAxisKey|MouseX`
  (params (AxisValue :type "Float (single-precision)"))
  ;[1 1 1] Mouse Control
)

(event `InputAxis|LeftRight`
  (params (AxisValue :type "Float (single-precision)"))
  ;[1 1 1] KeyboardControl
  (`self.K2_AddActorWorldOffset` (`KismetMathLibrary.MakeVector` 0.0 (* (* (`self.ScrollSpeed`) (`GameplayStatics.GetWorldDeltaSeconds`)) AxisValue))))

(event `InputAxis|TopDown`
  (params (AxisValue :type "Float (single-precision)"))
  ;[1 1 1] KeyboardControl
  (`self.K2_AddActorWorldOffset` (`KismetMathLibrary.MakeVector` (* (* (`self.ScrollSpeed`) (`GameplayStatics.GetWorldDeltaSeconds`)) AxisValue))))

(event `InputAxisKey|MouseY`
  (params (AxisValue :type "Float (single-precision)"))
  ;[1 1 1] Mouse Control
)

(fn `UserConstructionScript`)