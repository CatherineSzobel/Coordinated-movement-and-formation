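; HUD Blueprint that provides drag-box (marquee) selection of BP_BaseUnits actors.
; Pressed, hold and released events track mouse start and current positions and toggle drawing.
; While dragging, DrawHUD draws a translucent rectangle, queries actors inside it each frame, and messages units to select or deselect as SelectedUnits updates.
; Getter functions expose the selected units and their count.
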(event `/Game/Blueprints/BP_RTSInterface.Marquees Pressed`
  (bind (_locationx _locationy) (`PlayerController.GetMousePosition` (`GameplayStatics.GetPlayerController` 0)))
  ;[1 1 1] Marquee pressed
  (set `self.IsDrawing?` true)
  (bind _output_get (set `self.StartMousePos` (`KismetMathLibrary.MakeVector2D` _locationx _locationy)))
  (set `self.CurrentMousePos` _output_get))

(event `/Game/Blueprints/BP_RTSInterface.Marquees Hold`
  (bind (_locationx _locationy) (`PlayerController.GetMousePosition` (`GameplayStatics.GetPlayerController` 0)))
  ;[1 1 1] Marquee hold
  (set `self.CurrentMousePos` (`KismetMathLibrary.MakeVector2D` _locationx _locationy)))

(event `/Game/Blueprints/BP_RTSInterface.Marquees Released`
  ;[1 1 1] Marquee released
  (set `self.IsDrawing?` false))

(event `self.ReceiveDrawHUD`
  (params (SizeX :type Integer) (SizeY :type Integer))
  (bind (_startmousepos_x _startmousepos_y) (`KismetMathLibrary.BreakVector2D` (`self.StartMousePos`)))
  (bind (_currentmousepos_x _currentmousepos_y) (`KismetMathLibrary.BreakVector2D` (`self.CurrentMousePos`)))
  (bind _outactors (`self.GetActorsInSelectionRectangle` "/Game/Blueprints/BP_BaseUnits.BP_BaseUnits_C" (`self.StartMousePos`) (`self.CurrentMousePos`)))
  (if (`self.IsDrawing?`)
    (`self.DrawRect` (struct :`R` 0.277344 :`G` 0.566618 :`B` 0.75 :`A` 0.2) _startmousepos_x _startmousepos_y (- _currentmousepos_x _startmousepos_x) (- _currentmousepos_y _startmousepos_y))
    (set `self.ActorsInRectangle` _outactors)
    (for _array_element _outactors
      (message `/Game/Blueprints/BP_RTSInterface.Select Unit` _array_element)
      (`KismetArrayLibrary.Array_AddUnique` (`self.SelectedUnits`) _array_element))
    (for _array_element_2 (`self.SelectedUnits`)
      (if (== (`KismetArrayLibrary.Array_Find` (`self.ActorsInRectangle`) _array_element_2) -1)
        (message `/Game/Blueprints/BP_RTSInterface.Deselect Unit` _array_element_2)
        (`KismetArrayLibrary.Array_RemoveItem` (`self.SelectedUnits`) _array_element_2)))))

(fn `AmountOfUnits`
  (returns (Amount :type Integer))
  (return (`KismetArrayLibrary.Array_Length` (`self.SelectedUnits`))))

(fn `Grab Selected Units`
  (returns (Units :type "Array of Actor Object Reference"))
  (return (`self.SelectedUnits`)))

(fn `UserConstructionScript`)